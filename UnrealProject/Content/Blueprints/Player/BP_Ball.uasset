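; BP_Ball is a physics ball, apparently for pinball, that drives its own audio and frees itself when stuck.
; Each tick it feeds scaled speed into the audio component's BallSpeed parameter.
; If it is motionless before and after a delay, the sphere gets a random velocity-change impulse, equal on all axes.
; The impact-sound logic is disconnected, and the Hit and BallStuck events are empty.
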(event Custom|BallStuck)

(event EventTick
  (params (DeltaSeconds :type Float%20%28single-precision%29))
  (Audio|Parameter|SetFloatParameter (Variables|Default|GetAudio) "BallSpeed" (/ (Math|Vector|VectorLength (Transformation|GetVelocity)) 5e+03) :!class /Script/Engine.AudioComponent)
  (if (== (Math|Vector|VectorLength (Transformation|GetVelocity)) 0.0)
    (Utilities|FlowControl|Delay 1e+01)
    (if (== (Math|Vector|VectorLength (Transformation|GetVelocity)) 0.0)
      (Physics|AddImpulse (Variables|Default|GetSphere) (Math|Conversions|ToVector(Float) (Math|Random|RandomFloatinRange 3e+01 7e+01)) "None" true))))

(event Collision|EventHit
  (params (MyComp :type Primitive%20Component%20Object%20Reference) (Other :type Actor%20Object%20Reference) (OtherComp :type Primitive%20Component%20Object%20Reference) (bSelfMoved :type Boolean) (HitLocation :type Vector :default "0, 0, 0") (HitNormal :type Vector :default "0, 0, 0") (NormalImpulse :type Vector :default "0, 0, 0") (Hit :type Hit%20Result%20Structure%20%28by%20ref%29)))

(fn ConstructionScript)
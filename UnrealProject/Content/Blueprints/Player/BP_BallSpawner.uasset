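; BP_BallSpawner is a player-folder actor that launches a batch of BP_Ball actors from its location when play begins.
; On BeginPlay it loops over BallCount, spawning each ball at its own transform and adjusting position to avoid collisions.
; Each ball's Sphere gets a mass-independent impulse scaled by LaunchPower, in a random direction around the spawner's up axis.
; Every spawn also calls AddLifeMessage on the game instance.
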(event EventBeginPlay
  (for _index (range 0 (Variables|Default|GetBallCount))
    (bind _returnvalue (Game|SpawnActorfromClass "/Game/Blueprints/Player/BP_Ball.BP_Ball_C" (Transformation|GetActorTransform) "AdjustIfPossibleButAlwaysSpawn" "MultiplyWithRoot" 0 0))
    (Physics|AddImpulse (Variables|/Game/Blueprints/Player/BP_Ball.BP_Ball_C|GetSphere _returnvalue) (* (Math|Vector|RotateVectorAroundAxis (Transformation|GetActorForwardVector) (Math|Random|RandomFloatinRange 0.0 3.6e+02) (Transformation|GetActorUpVector)) (Variables|Default|GetLaunchPower)) "None" true)
    (Class|BPIScore|AddLife(Message) (Game|GetGameInstance))))

(fn ConstructionScript)
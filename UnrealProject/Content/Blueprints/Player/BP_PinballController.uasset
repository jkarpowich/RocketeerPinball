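; Player controller for a pinball game that owns the main and pause menus and routes Enhanced Input to the table.
; On BeginPlay it creates both widgets, adds the input context, polls each tick until key mappings load for the menu, and finds tagged paddles and the launcher.
; Input flips paddles, converts hold time into clamped launch power, and toggles pause outside the main menu.
; UpdateMapping rebinds keys on the mapping context.
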(event Custom|UpdateMapping
  (params (Action :type Input%20Action%20Object%20Reference) (Key :type Key%20Structure :default "None"))
  (for _array_element (Variables|Default|GetMappings)
    (if (== (.action _array_element) Action)
      (Class|InputMappingContext|UnmapKey (Variables|Default|GetMapping%20Context) Action (.key _array_element))
      (Class|InputMappingContext|MapKey (Variables|Default|GetMapping%20Context) Action Key))))

(event Input|EnhancedActionEvents|EnhancedInputActionIA_PaddleLeft
  (params (ActionValue :type Boolean) (ElapsedSeconds :type Float%20%28double-precision%29) (TriggeredSeconds :type Float%20%28double-precision%29) (InputAction :type Input%20Action%20Object%20Reference :default "/Game/Input/IA_PaddleLeft.IA_PaddleLeft"))
  (:Started
    (Default|FlipEvent (Variables|Default|GetLeftPaddle)))
  (:Completed
    (Default|UnflipEvent (Variables|Default|GetLeftPaddle))))

(event Input|EnhancedActionEvents|EnhancedInputActionIA_PaddleRight
  (params (ActionValue :type Boolean) (ElapsedSeconds :type Float%20%28double-precision%29) (TriggeredSeconds :type Float%20%28double-precision%29) (InputAction :type Input%20Action%20Object%20Reference :default "/Game/Input/IA_PaddleRight.IA_PaddleRight"))
  (:Started
    (Default|FlipEvent (Variables|Default|GetRightPaddle)))
  (:Completed
    (Default|UnflipEvent (Variables|Default|GetRightPaddle))))

(event Input|EnhancedActionEvents|EnhancedInputActionIA_Launch
  (params (ActionValue :type Boolean) (ElapsedSeconds :type Float%20%28double-precision%29) (TriggeredSeconds :type Float%20%28double-precision%29) (InputAction :type Input%20Action%20Object%20Reference :default "/Game/Input/IA_Launch.IA_Launch"))
  (:Triggered
    (Default|UpdateCharge (Variables|Default|GetLauncher) (CallFunction|LaunchPower TriggeredSeconds)))
  (:Completed
    (Default|LaunchEvent (Variables|Default|GetLauncher) (CallFunction|LaunchPower ElapsedSeconds))))

(event Input|EnhancedActionEvents|EnhancedInputActionIA_Pause
  (params (ActionValue :type Boolean) (ElapsedSeconds :type Float%20%28double-precision%29) (TriggeredSeconds :type Float%20%28double-precision%29) (InputAction :type Input%20Action%20Object%20Reference :default "/Game/Input/IA_Pause.IA_Pause"))
  (:Started
    (if (not (UserInterface|Viewport|IsinViewport (Variables|Default|GetMainMenuWidget)))
      (if (Game|IsGamePaused)
        (Default|FadeOut (Variables|Default|GetPauseWidget))
        (Game|SetGamePaused false)
        (Variables|/Script/Engine.PlayerController|SetbShowMouseCursor self false)
        (Input|SetInputModeGameOnly self false)
        (else
          (Default|Fadein (Variables|Default|GetPauseWidget))
          (Game|SetGamePaused true)
          (Variables|/Script/Engine.PlayerController|SetbShowMouseCursor self true)
          (Input|SetInputModeUIOnly self (Variables|Default|GetPauseWidget) "DoNotLock" false))))))

(event EventBeginPlay
  (bind _self self)
  (bind _returnvalue (PlayerController|LocalPlayerSubsystems|GetEnhancedInputLocalPlayerSubsystem _self))
  (bind _returnvalue_2 (Class|EnhancedInputSubsystemInterface|GetAllPlayerMappableActionKeyMappings _returnvalue))
  (Utilities|FlowControl|Sequence
    (:then_0
      (bind _returnvalue_3 (UserInterface|CreateWidget "/Game/UI/Menus/W_Menu.W_Menu_C"))
      (bind _output_get (Variables|Default|SetMainMenuWidget _returnvalue_3))
      (UserInterface|Viewport|AddtoViewport _output_get 0)
      (bind _returnvalue_4 (UserInterface|CreateWidget "/Game/UI/Menus/W_PauseMenu.W_PauseMenu_C" (Game|GetPlayerController 0)))
      (Variables|Default|SetPauseWidget _returnvalue_4))
    (:then_1
      (Utilities|IsValid _returnvalue
        (:Is%20Valid
          (Input|AddMappingContext _returnvalue "/Game/Input/IMC_Input.IMC_Input" 0 "(bIgnoreAllPressedKeysUntilRelease=True,bForceImmediately=False,bNotifyUserSettings=False)")
          (if (Utilities|Array|IsNotEmpty _returnvalue_2) :!label _label
            (bind _output_get_2 (Variables|Default|SetMappings _returnvalue_2))
            (Default|RefreshMappings (Variables|Default|GetMainMenuWidget) _output_get_2)
            (else
              (Utilities|FlowControl|DelayUntilNextTick)
              (goto _label))))))
    (:then_2
      (bind _outactors (Actor|GetAllActorsOfClasswithTag "/Game/Blueprints/Machine/BP_Paddle.BP_Paddle_C" "left"))
      (Variables|Default|SetLeftPaddle (Utilities|Array|Get(acopy) _outactors))
      (bind _outactors_2 (Actor|GetAllActorsOfClasswithTag "/Game/Blueprints/Machine/BP_Paddle.BP_Paddle_C" "right"))
      (Variables|Default|SetRightPaddle (Utilities|Array|Get(acopy) _outactors_2)))
    (:then_3
      (bind _returnvalue_5 (Actor|GetActorOfClass "/Game/Blueprints/Machine/BP_Launcher.BP_Launcher_C"))
      (Variables|Default|SetLauncher _returnvalue_5))))

(fn ConstructionScript)

(fn LaunchPower
  (params (Time :type Float%20%28double-precision%29))
  (return (Math|Float|MapRangeClamped Time 0.0 (Variables|Default|GetMax%20Ball%20Charge%20Time) 0.0 1.0)))
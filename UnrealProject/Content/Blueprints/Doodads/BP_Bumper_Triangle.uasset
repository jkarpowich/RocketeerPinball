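; Triangular pinball-style bumper that knocks a BP_Ball away and awards score when it hits the bumper face aligned with the Arrow component.
; Box hits compare the absolute normal to the arrow's absolute forward vector, then apply a velocity-change impulse from FollowArrow.
; A valid hit also plays a sound and a timeline-driven material Scale pulse.
; A DoOnce with a short delayed reset debounces repeated hits.
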(event OnComponentHit(Box)
  (params (HitComponent :type Primitive%20Component%20Object%20Reference) (OtherActor :type Actor%20Object%20Reference) (OtherComp :type Primitive%20Component%20Object%20Reference) (NormalImpulse :type Vector :default "0, 0, 0") (Hit :type Hit%20Result%20Structure%20%28by%20ref%29))
  (bind _asbp_ball (Utilities|Casting|CastToBP_Ball OtherActor))
  (if (Utilities|Operators|EqualEqual (Math|Vector|VectorGetAbs (.normal Hit)) (Math|Vector|VectorGetAbs (Math|Vector|GetForwardVector (Variables|Default|GetArrow))) 0.01)
    (Utilities|FlowControl|DoOnce false :!label _label
      (:Completed
        (Physics|AddImpulse (Variables|/Game/Blueprints/Player/BP_Ball.BP_Ball_C|GetSphere _asbp_ball) (|Followarrow) "None" true)
        (Class|BPIScore|AddScore(Message) (Game|GetGameInstance) (Variables|Default|GetScore))
        (Utilities|FlowControl|Sequence
          (:then_0
            (bind _scale (Timeline|Timeline PlayFromStart)
              (:Update
                (Rendering|Material|SetScalarParameterValueonMaterials (Variables|Default|GetStaticMesh) "Scale" _scale))))
          (:then_1
            (Audio|PlaySoundatLocation (Variables|Default|GetSound) (Transformation|GetActorLocation) (Transformation|GetActorRotation) 1.0 1.0 0.0 0 0 0 0))
          (:then_2
            (Utilities|FlowControl|Delay 0.2)
            (goto _label Reset)))))))

(event EventBeginPlay)

(event Collision|EventActorBeginOverlap
  (params (OtherActor :type Actor%20Object%20Reference)))

(event EventTick
  (params (DeltaSeconds :type Float%20%28single-precision%29)))

(fn ConstructionScript)
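; GI_Pinball is the pinball game's Game Instance, tracking score, lives and high score, plus music and master volume.
; AddScore applies a combo multiplier that expires via a retriggerable delay; reaching the replay score zeroes the score and grants a life.
; Losing the last life resets state, shows the play-again widget and stops the MetaSound music by trigger.
; High score and sound-mix volume persist through an asynchronously loaded and saved SaveGame.
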(event Custom|Save%20Game
  (|AsyncSaveGametoSlot (Variables|Default|GetSaveGame) "Highscore"))

(event EventAddScore
  (params (Score :type Integer))
  (bind _output_get (Variables|Default|SetLastScore (* Score (Variables|Default|GetCombo))))
  (Variables|Default|SetScore (+ _output_get (Variables|Default|GetScore)))
  (CallFunction|UpdateHighScore)
  (Utilities|FlowControl|Sequence
    (:then_0
      (if (>= (Variables|Default|GetScore) (Variables|Default|GetReplayScore))
        (Variables|Default|SetScore 0)
        (CallFunction|AddLife)))
    (:then_1
      (Math|Integer|IncrementInt (Variables|Default|GetCombo)
        (:%20%20
          (Utilities|FlowControl|RetriggerableDelay 2.0)
          (Variables|Default|SetCombo 1))))))

(event EventAddLife
  (Math|Integer|IncrementInt (Variables|Default|GetLives)))

(event EventRemoveLife
  (Math|Integer|DecrementInt (Variables|Default|GetLives)
    (:%20%20
      (if (== (Variables|Default|GetLives) 0)
        (CallFunction|Reset)
        (Audio|PlaySound2D "/Game/Audio/SFX/EndOfGame.EndOfGame" 1.0 1.0 0.0 0 0)
        (bind _returnvalue (UserInterface|CreateWidget "/Game/UI/Menus/W_PlayAgain.W_PlayAgain_C"))
        (UserInterface|Viewport|AddtoViewport _returnvalue 0)
        (CallFunction|StopMusic)))))

(event EventInit
  (bind (_savegame _bsuccess) (|AsyncLoadGamefromSlot "Highscore")
    (:Completed
      (if _bsuccess
        (bind _asbp_save_game (Utilities|Casting|CastToBP_SaveGame _savegame))
        (bind _output_get (Variables|Default|SetSaveGame _asbp_save_game))
        (Variables|Default|SetHighScore (Variables|/Game/Blueprints/BP_SaveGame.BP_SaveGame_C|GetHighscore _output_get))
        (else
          (bind _returnvalue (SaveGame|CreateSaveGameObject "/Game/Blueprints/BP_SaveGame.BP_SaveGame_C"))
          (Variables|Default|SetSaveGame _returnvalue)
          (CallFunction|SaveGame)))
      (CallFunction|UpdateVolume (Variables|/Game/Blueprints/BP_SaveGame.BP_SaveGame_C|GetVolume (Variables|Default|GetSaveGame)))
      (bind _returnvalue_2 (Audio|CreateSound2D "/Game/Audio/Music/MS_Music.MS_Music" 1.0 1.0 0.0 0 true false))
      (Variables|Default|SetMusic _returnvalue_2))))

(event EventUpdateVolume
  (params (Vol :type Float%20%28double-precision%29))
  (bind _output_get (Variables|/Game/Blueprints/BP_SaveGame.BP_SaveGame_C|SetVolume (Variables|Default|GetSaveGame) Vol))
  (Audio|SetSoundMixClassOverride "/Game/Audio/SCM_Master.SCM_Master" "/Game/Audio/SC_All.SC_All" _output_get 1.0 1.0 true)
  (Audio|PushSoundMixModifier "/Game/Audio/SCM_Master.SCM_Master")
  (CallFunction|SaveGame))

(event EventStartMusic
  (Audio|Components|Audio|Play (Variables|Default|GetMusic) 0.0))

(event EventStopMusic
  (Class|AudioParameterControllerInterface|SetTriggerParameter (Variables|Default|GetMusic) "StopMusic"))

(fn UpdateHighScore
  (bind _output_get (Variables|Default|SetHighScore (Math|Integer|SelectInt (Variables|Default|GetScore) (Variables|Default|GetHighScore) (> (Variables|Default|GetScore) (Variables|Default|GetHighScore)))))
  (Variables|/Game/Blueprints/BP_SaveGame.BP_SaveGame_C|SetHighscore (Variables|Default|GetSaveGame) _output_get)
  (CallFunction|SaveGame))

(fn Reset
  (Variables|Default|SetScore 0)
  (Variables|Default|SetLives 5)
  (Variables|Default|SetCombo 1))

(fn GetVolume
  (return (Variables|/Game/Blueprints/BP_SaveGame.BP_SaveGame_C|GetVolume (Variables|Default|GetSaveGame))))
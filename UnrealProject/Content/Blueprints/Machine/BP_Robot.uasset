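; BP_Robot is an animated robot that returns the ball after it falls in the gutter and celebrates wins.
; BeginPlay caches BP_Ball's starting location and binds to BP_Gutter's overlap event.
; A gutter overlap plays a restart montage showing a prop ball mesh, then teleports the ball back, zeroes its velocity and plays a sound.
; A separate event plays the winning montage, with DoOnce gates blocking retriggers until each montage completes.
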(event Custom|PlayWinAnimation_Event
  (Utilities|FlowControl|DoOnce false :!label _label
    (:Completed
      (Animation|Montage|PlayMontage (Variables|Default|GetSkeletalMesh) "/Game/Animations/Robot/MTG_Winning.MTG_Winning" 1.5
        (:OnCompleted
          (goto _label Reset))))))

(event Custom|InGutter
  (params (OverlappedActor :type Actor%20Object%20Reference) (OtherActor :type Actor%20Object%20Reference))
  (Utilities|FlowControl|DoOnce false :!label _label
    (:Completed
      (Animation|Montage|PlayMontage (Variables|Default|GetSkeletalMesh) "/Game/Animations/Robot/MTG_RobotRestart.MTG_RobotRestart" 1.5
        (:then
          (Development|SetHiddeninGame (Variables|Default|GetBallMesh) false false))
        (:OnCompleted
          (Transformation|SetActorLocation (Variables|Default|GetBall) (Variables|Default|GetSpawnLocation) false true)
          (Physics|SetPhysicsLinearVelocity (Variables|/Game/Blueprints/Player/BP_Ball.BP_Ball_C|GetSphere (Variables|Default|GetBall)) "0, 0, 0" false "None")
          (Development|SetHiddeninGame (Variables|Default|GetBallMesh) true false)
          (Audio|PlaySoundatLocation "/Game/Audio/SFX/BallReturn.BallReturn" (Variables|Default|GetSpawnLocation) "0, 0, 0" 1.0 1.0 0.0 0 0 0 0)
          (goto _label Reset))))))

(event EventBeginPlay
  (Utilities|FlowControl|Sequence
    (:then_0
      (bind _returnvalue (Actor|GetActorOfClass "/Game/Blueprints/Player/BP_Ball.BP_Ball_C"))
      (bind _output_get (Variables|Default|SetBall _returnvalue))
      (Variables|Default|SetSpawnLocation (Transformation|GetActorLocation _output_get)))
    (:then_1
      (bind _returnvalue_2 (Actor|GetActorOfClass "/Game/Blueprints/Machine/BP_Gutter.BP_Gutter_C"))
      (bind _output_get_2 (Variables|Default|SetGutter _returnvalue_2))
      (Collision|BindEventtoOnActorBeginOverlap _output_get_2 (EventDispatchers|CreateEvent :!event Custom|InGutter)))))

(fn ConstructionScript)
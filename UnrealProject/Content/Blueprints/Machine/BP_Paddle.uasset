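; BP_Paddle is a flipper that rotates to strike BP_Ball, apparently in a pinball-style machine.
; Flip and unflip events set the target yaw and a Hitting flag, with flipping also playing a sound.
; Tick eases the flipper mesh's relative yaw toward that target with FInterpTo.
; Ball hits while flipping enter a DoOnce reset after a short delay, with no other effect.
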(event OnComponentHit(SM_Flipper)
  (params (HitComponent :type Primitive%20Component%20Object%20Reference) (OtherActor :type Actor%20Object%20Reference) (OtherComp :type Primitive%20Component%20Object%20Reference) (NormalImpulse :type Vector :default "0, 0, 0") (Hit :type Hit%20Result%20Structure%20%28by%20ref%29))
  (Utilities|Casting|CastToBP_Ball OtherActor)
  (if (Variables|Default|GetHitting)
    (Utilities|FlowControl|DoOnce false :!label _label
      (:Completed
        (Utilities|FlowControl|Delay 0.2)
        (goto _label Reset)))))

(event Custom|Flip_Event
  (Variables|Default|SetTargetPosition (Variables|Default|GetFlipped%20Yaw))
  (Variables|Default|SetHitting true)
  (Audio|PlaySoundatLocation (Variables|Default|GetSound) (Transformation|GetActorLocation) "0, 0, 0" 1.0 1.0 0.0 0 0 0 0))

(event Custom|Unflip_Event
  (Variables|Default|SetTargetPosition 0.0)
  (Variables|Default|SetHitting false))

(event EventBeginPlay)

(event EventTick
  (params (DeltaSeconds :type Float%20%28single-precision%29))
  (bind _output_get (Variables|Default|SetRelativeYaw (Math|Interpolation|FInterpTo (Variables|Default|GetRelativeYaw) (Variables|Default|GetTargetPosition) (Utilities|Time|GetWorldDeltaSeconds) (Variables|Default|GetPaddle%20Speed))))
  (Transformation|SetRelativeRotation (Variables|Default|GetSM_Flipper) (Math|Rotator|MakeRotator 0.0 0.0 _output_get) false false))

(fn ConstructionScript)
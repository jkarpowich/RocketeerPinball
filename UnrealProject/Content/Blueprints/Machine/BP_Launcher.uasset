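; Launcher machine actor that fires the level's BP_Ball along its arrow when the ball overlaps it.
; UpdateCharge feeds the charge percent to a W_Launcher widget and the MPC_Global BlinkRate parameter, starting the charge audio if needed.
; Launch_Event resets the charge, then applies a power-squared velocity impulse and triggers the launch sound, or stops audio without a ball.
; A DoOnce reset after a short delay prevents repeated launches.
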(event Custom|Launch_Event
  (params (Power :type Float%20%28double-precision%29))
  (CallFunction|UpdateCharge 0.0)
  (if (CallFunction|HasBall)
    (Utilities|FlowControl|DoOnce false :!label _label
      (:Completed
        (Physics|AddImpulse (Variables|/Game/Blueprints/Player/BP_Ball.BP_Ball_C|GetSphere (Variables|Default|GetBall)) (* Power (Variables|Default|GetPower) (Math|Vector|GetForwardVector (Variables|Default|GetArrow))) "None" true)
        (Class|AudioParameterControllerInterface|SetTriggerParameter (Variables|Default|GetAudio) "Launch")
        (Variables|Default|SetAudioPlaying false)
        (Utilities|FlowControl|Delay 0.3)
        (goto _label Reset)))
    (else
      (Audio|Components|Audio|Stop (Variables|Default|GetAudio))
      (Variables|Default|SetAudioPlaying false))))

(event EventBeginPlay
  (bind _returnvalue (Actor|GetActorOfClass "/Game/Blueprints/Player/BP_Ball.BP_Ball_C"))
  (Variables|Default|SetBall _returnvalue)
  (bind _asw_launcher (Utilities|Casting|CastToW_Launcher (UserInterface|GetUserWidgetObject (Variables|Default|GetWidget))))
  (Variables|Default|SetChargeWidget _asw_launcher)
  (Audio|Components|Audio|Stop (Variables|Default|GetAudio)))

(fn ConstructionScript)

(fn HasBall
  (return (Collision|IsOverlappingActor (Variables|Default|GetBall) :!class /Script/Engine.Actor)))

(fn UpdateCharge
  (params (Percent :type Float%20%28double-precision%29))
  (bind _output_get (Variables|/Game/UI/Machine/W_Launcher.W_Launcher_C|SetPercent (Variables|Default|GetChargeWidget) Percent))
  (Rendering|Material|SetScalarParameterValue "/Game/Materials/MPC_Global.MPC_Global" "BlinkRate" (* _output_get 2.5) :!class /Script/Engine.KismetMaterialLibrary)
  (if (not (Variables|Default|GetAudioPlaying))
    (Audio|Components|Audio|Play (Variables|Default|GetAudio) 0.0)
    (Variables|Default|SetAudioPlaying true)))
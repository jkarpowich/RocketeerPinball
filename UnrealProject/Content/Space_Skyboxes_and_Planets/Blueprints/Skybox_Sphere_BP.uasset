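; Skybox sphere actor that configures a space sky material from its editable properties.
; The construction script writes brightness, power and rotation to the Skybox_Parameters collection, creates a dynamic material instance and calls RefreshMaterial; a bool acts as a re-run button.
; RefreshMaterial takes sun direction and color from an assigned directional light, otherwise derives them from SunHeight and actor yaw.
; UpdateSunDirection pushes the light's direction, color and height to the material.
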(fn ConstructionScript
  ;[1 1 1] Skybox base
  (Rendering|Material|SetMaterial (Variables|Default|GetStaticMesh) 0 (Variables|Default|GetMaterial%20Instanced))
  ;[1 1 1] Customization parameters
  (Rendering|Material|SetScalarParameterValue "/Game/Space_Skyboxes_and_Planets/Blueprints/Skybox_Parameters.Skybox_Parameters" "Star Brightness" (Variables|Default|GetStar%20Brightness) :!class /Script/Engine.KismetMaterialLibrary)
  (Rendering|Material|SetScalarParameterValue "/Game/Space_Skyboxes_and_Planets/Blueprints/Skybox_Parameters.Skybox_Parameters" "Power" (Variables|Default|GetPower) :!class /Script/Engine.KismetMaterialLibrary)
  (Rendering|Material|SetScalarParameterValue "/Game/Space_Skyboxes_and_Planets/Blueprints/Skybox_Parameters.Skybox_Parameters" "Scene Brightness" (Variables|Default|GetScene%20Brightness) :!class /Script/Engine.KismetMaterialLibrary)
  ;[1 1 1] Rotation parameters
  (Rendering|Material|SetScalarParameterValue "/Game/Space_Skyboxes_and_Planets/Blueprints/Skybox_Parameters.Skybox_Parameters" "X Rotation" (Variables|Default|GetX%20Rotation) :!class /Script/Engine.KismetMaterialLibrary)
  (Rendering|Material|SetScalarParameterValue "/Game/Space_Skyboxes_and_Planets/Blueprints/Skybox_Parameters.Skybox_Parameters" "Y Rotation" (Variables|Default|GetY%20Rotation) :!class /Script/Engine.KismetMaterialLibrary)
  (Rendering|Material|SetScalarParameterValue "/Game/Space_Skyboxes_and_Planets/Blueprints/Skybox_Parameters.Skybox_Parameters" "Z Rotation" (Variables|Default|GetZ%20Rotation) :!class /Script/Engine.KismetMaterialLibrary)
  (bind _returnvalue (Rendering|Material|CreateDynamicMaterialInstance (Variables|Default|GetStaticMesh) 0 0 "None" :!class /Script/Engine.PrimitiveComponent))
  (Variables|Default|SetSky%20material _returnvalue)
  (if (Variables|Default|GetRefresh%20material) ; Updating bool in details panel causes construction script to run again
    _
    (else
      _))
  (Variables|Default|SetRefresh%20material false)
  (CallFunction|RefreshMaterial))

(fn UpdateSunDirection
  (bind _sky_material (Variables|Default|GetSky%20material))
  (Rendering|Material|SetVectorParameterValue _sky_material "Light direction" (Math|Conversions|ToLinearColor(Vector) (Math|Rotator|GetRotationXVector (Transformation|GetActorRotation (Variables|Default|GetDirectional%20light%20actor)))) :!class /Script/Engine.MaterialInstanceDynamic)
  (Rendering|Material|SetVectorParameterValue _sky_material "Sun color" (Math|Conversions|ToLinearColor(Color) (Variables|/Script/Engine.LightComponentBase|GetLightColor (Variables|/Script/Engine.Light|GetLightComponent (Variables|Default|GetDirectional%20light%20actor)))) :!class /Script/Engine.MaterialInstanceDynamic)
  (Variables|Default|SetSun%20height (Math|Float|MapRangeUnclamped (.Pitch (Math|Rotator|BreakRotator (Transformation|GetActorRotation (Variables|Default|GetDirectional%20light%20actor)))) 0.0 -9e+01 0.0 1.0))
  (Rendering|Material|SetScalarParameterValue (Variables|Default|GetSky%20material) "Sun height" (Variables|Default|GetSun%20height) :!class /Script/Engine.MaterialInstanceDynamic))

(fn RefreshMaterial
  (bind _sky_material (Variables|Default|GetSky%20material))
  (bind _sky_material_2 (Variables|Default|GetSky%20material))
  (Utilities|IsValid (Variables|Default|GetDirectional%20light%20actor) ; Has a directional light been assigned?
    (:Is%20Valid
      (Rendering|Material|SetVectorParameterValue _sky_material_2 "Light direction" (Math|Conversions|ToLinearColor(Vector) (Math|Rotator|GetRotationXVector (Transformation|GetActorRotation (Variables|Default|GetDirectional%20light%20actor)))) :!class /Script/Engine.MaterialInstanceDynamic)
      (Rendering|Material|SetVectorParameterValue _sky_material_2 "Sun color" (Math|Conversions|ToLinearColor(Color) (Variables|/Script/Engine.LightComponentBase|GetLightColor (Variables|/Script/Engine.Light|GetLightComponent (Variables|Default|GetDirectional%20light%20actor)))) :!class /Script/Engine.MaterialInstanceDynamic)
      (Variables|Default|SetSun%20height (Math|Float|MapRangeUnclamped (.Pitch (Math|Rotator|BreakRotator (Transformation|GetActorRotation (Variables|Default|GetDirectional%20light%20actor)))) 0.0 -9e+01 0.0 1.0)))
    (:Is%20Not%20Valid
      (Rendering|Material|SetVectorParameterValue _sky_material "Light direction" (Math|Conversions|ToLinearColor(Vector) (Math|Rotator|GetRotationXVector (Math|Rotator|MakeRotator 0.0 (Math|Float|MapRangeUnclamped (Variables|Default|GetSun%20height) -1.0 1.0 9e+01 -9e+01) (.Yaw (Math|Rotator|BreakRotator (Transformation|GetActorRotation)))))) :!class /Script/Engine.MaterialInstanceDynamic)
      (Rendering|Material|SetVectorParameterValue _sky_material "Sun color" (Math|Color|Lerp(LinearColor) "(R=1.000000,G=0.221000,B=0.040000,A=1.000000)" "(R=0.954000,G=0.901000,B=0.744120,A=1.000000)" (Math|Float|Clamp(Float) (+ (Variables|Default|GetSun%20height) 0.2))) :!class /Script/Engine.MaterialInstanceDynamic))))